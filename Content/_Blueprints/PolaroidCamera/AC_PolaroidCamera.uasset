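; Polaroid camera component that captures in-game photos to disk and toggles a photo gallery.
; TakePhoto renders the given scene capture to a new render target, exports it under the project's Photos folder with a timestamped name, and plays a shutter sound.
; It then appends the filename to the SG_Photos save, creating that save if missing.
; ToggleGallery adds or removes W_PhotoGallery, switching input mode and mouse cursor.
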(event `TakePhoto`
  (params (SceneCapture :type "SceneCaptureComponent2D Object Reference"))
  (bind (_returnvalue_year _returnvalue_month _returnvalue_day _returnvalue_hour _returnvalue_minute _returnvalue_second) (`KismetMathLibrary.BreakDateTime` (`KismetMathLibrary.Now`)))
  (bind _returnvalue (`KismetRenderingLibrary.CreateRenderTarget2D` 256))
  (bind _output_get (set `SceneCaptureComponent2D.TextureTarget` _returnvalue SceneCapture))
  (`SceneCaptureComponent2D.CaptureScene` SceneCapture)
  (`KismetSystemLibrary.Delay` 0.2)
  (bind _output_get_2 (set `self.Photo` _output_get))
  (bind _output_get_3 (set `self.FileName` (`KismetTextLibrary.Conv_TextToString` (`|FormatText` "PalaeoCam{DD}{MM}{YYYY}{HH}{MI}{SS}" (`KismetTextLibrary.Conv_IntToText` _returnvalue_day false false 2) (`KismetTextLibrary.Conv_IntToText` _returnvalue_month false false 2) (`KismetTextLibrary.Conv_IntToText` _returnvalue_year false false 2) (`KismetTextLibrary.Conv_IntToText` _returnvalue_hour false false 2) (`KismetTextLibrary.Conv_IntToText` _returnvalue_minute false false 2) (`KismetTextLibrary.Conv_IntToText` _returnvalue_second false false 2)))))
  ;[0 0.02037 0.15 0.5] export photo to directory
  (`KismetRenderingLibrary.ExportRenderTarget` _output_get_2 (`KismetStringLibrary.Concat_StrStr` (`KismetSystemLibrary.GetProjectDirectory`) "Photos/") _output_get_3)
  (set `self.Photo` null)
  (`GameplayStatics.PlaySound2D` "/Game/_Audio/S_CameraShutter.S_CameraShutter" 1.0 1.0 0.0 null null)
  ;[0.01577 0.02706 0.15 0.5] Save photo and add it to the list of saved photos
  (bind _returnvalue_2 (`GameplayStatics.DoesSaveGameExist` "SG_Photos"))
  (if _returnvalue_2
    (bind _returnvalue_3 (`GameplayStatics.LoadGameFromSlot` "SG_Photos"))
    (bind _assg_photos (cast `/Game/_Blueprints/PolaroidCamera/SG_Photos` _returnvalue_3))
    (bind _output_get_4 (set `self.As SG Photos` _assg_photos))
    (`KismetArrayLibrary.Array_Add` (`/Game/_Blueprints/PolaroidCamera/SG_Photos.PhotoFileNames` _output_get_4) (`self.FileName`))
    (else
      (bind _returnvalue_4 (`GameplayStatics.CreateSaveGameObject` "/Game/_Blueprints/PolaroidCamera/SG_Photos.SG_Photos_C"))
      (bind _output_get_5 (set `self.As SG Photos` _returnvalue_4))
      (`KismetArrayLibrary.Array_Add` (`/Game/_Blueprints/PolaroidCamera/SG_Photos.PhotoFileNames` _output_get_5) (`self.FileName`))))
  (`GameplayStatics.SaveGameToSlot` (`self.As SG Photos`) "SG_Photos"))

(event `ToggleGallery`
  (bind _returnvalue (`GameplayStatics.GetPlayerController` 0))
  (bind _returnvalue_2 (`GameplayStatics.GetPlayerController` 0))
  ;[0.01114 0.0441 0.15 0.5] toggle gallery
  (bind _photogallery (`self.PhotoGallery`)
    (:`then`
      (`Widget.RemoveFromParent` _photogallery)
      (set `self.PhotoGallery` null)
      (`WidgetBlueprintLibrary.SetInputMode_GameOnly` _returnvalue)
      (set `PlayerController.bShowMouseCursor` false _returnvalue))
    (:`else`
      (bind _returnvalue_3 (`|CreateWidget` "/Game/_Blueprints/PolaroidCamera/W_PhotoGallery.W_PhotoGallery_C"))
      (bind _output_get (set `self.PhotoGallery` _returnvalue_3))
      (`UserWidget.AddToViewport` _output_get 0)
      (`WidgetBlueprintLibrary.SetInputMode_GameAndUIEx` _returnvalue_2 _output_get)
      (set `PlayerController.bShowMouseCursor` true _returnvalue_2))))