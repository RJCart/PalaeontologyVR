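; Fossil placement puzzle Blueprint that registers fossil pieces dropped onto their matching placement zones.
; Three overlap events compare the actor to piece references, then set a correct flag, play a drop sound and reveal that piece's component.
; AllPiecesCorrect checks five flags but is never called here.
; PlaySequence starts the Quetz landscape end sequence without checking completion; several other helper functions are stubs.
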(event `self.Placement_Piece01.OnComponentBeginOverlap`
  (params (OverlappedComponent :type "PrimitiveComponent Object Reference") (OtherActor :type "Actor Object Reference") (OtherComp :type "PrimitiveComponent Object Reference") (OtherBodyIndex :type Integer) (bFromSweep :type Boolean) (SweepResult :type "HitResult Structure (by ref)"))
  (if (== OtherActor (`self.Piece1Reference`))
    (set `self.Piece1IsCorrect` true)
    (`GameplayStatics.PlaySound2D` (`self.DropSound`) 1.0 1.0 0.0 null null)
    (`SceneComponent.SetVisibility` (`self.Piece_01`) true false)
    (set `self.Piece1Visibility` true)))

(event `self.Placement_Piece02.OnComponentBeginOverlap`
  (params (OverlappedComponent :type "PrimitiveComponent Object Reference") (OtherActor :type "Actor Object Reference") (OtherComp :type "PrimitiveComponent Object Reference") (OtherBodyIndex :type Integer) (bFromSweep :type Boolean) (SweepResult :type "HitResult Structure (by ref)"))
  (if (== OtherActor (`self.Piece2Reference`))
    (set `self.Piece2IsCorrect` true)
    (`GameplayStatics.PlaySound2D` (`self.DropSound`) 1.0 1.0 0.0 null null)
    (`SceneComponent.SetVisibility` (`self.Piece_02`) true false)
    (set `self.Piece2Visibility` true)))

(event `self.Placement_Piece03.OnComponentBeginOverlap`
  (params (OverlappedComponent :type "PrimitiveComponent Object Reference") (OtherActor :type "Actor Object Reference") (OtherComp :type "PrimitiveComponent Object Reference") (OtherBodyIndex :type Integer) (bFromSweep :type Boolean) (SweepResult :type "HitResult Structure (by ref)"))
  (if (== OtherActor (`self.Piece3Reference`))
    (set `self.Piece3IsCorrect` true)
    (`GameplayStatics.PlaySound2D` (`self.DropSound`) 1.0 1.0 0.0 null null)
    (`SceneComponent.SetVisibility` (`self.Piece_03`) true false)
    (set `self.Piece3Visibility` true)))

(event `Play Sequence`
  ;[0.06339 0.07131 0.15 0.5] If All Pieces correct play end sequence
  (if true
    (`LevelSequencePlayer.CreateLevelSequencePlayer` "/Game/_Art/Animation/AnimationSequence/LS_Quetz_Landscape_01.LS_Quetz_Landscape_01")
    (`MovieSceneSequencePlayer.Play` (`LevelSequenceActor.SequencePlayer` (`self.EndSequence`)))))

(fn `AdvancePuzzle`
  (bind _output_get (set `self.PuzzleStage` (+ (`self.PuzzleStage`) 1)))
  (`KismetSystemLibrary.PrintString` (`KismetStringLibrary.Conv_IntToString` _output_get)))

(fn `AllPiecesCorrect`
  (if (and (`self.Piece1IsCorrect`) (`self.Piece2IsCorrect`) (`self.Piece3IsCorrect`) (`self.Piece4IsCorrect`) (`self.Piece5IsCorrect`))
    (set `self.IsPuzzleComplete` true)))

(fn `Piece1Correct`
  (returns (Piece1Correct :type Boolean))
  (return false))

(fn `Piece2Correct`
  (returns (Piece2Correct :type Boolean))
  (return false))

(fn `PieceInPlace`
  (params (A :type "Object Object Reference") (B :type "Object Object Reference"))
  (if (== A B)
    (set `self.Piece1IsCorrect` true)))

(fn `PieceOutOfPlace`
  (params (A :type "Object Object Reference") (B :type "Object Object Reference"))
  (if (== A B)
    (set `self.Piece1IsCorrect` false)))

(fn `PuzzleWorldLocation`
  (params (PuzzleLocationIn :type "Vector Structure" :default (0.0 0.0 0.0)))
  (returns (PuzzleLocationOut :type "Vector Structure"))
  (return (0.0 0.0 0.0)))

(fn `Slot1Filled`
  (params (Slot1Filled :type Boolean :default false))
  (returns (Slot1IsFilled :type Boolean))
  (return Slot1Filled))

(fn `UserConstructionScript`)