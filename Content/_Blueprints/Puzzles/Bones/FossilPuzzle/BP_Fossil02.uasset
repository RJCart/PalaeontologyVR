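; BP_Fossil02 is a piece in the bone fossil puzzle that reacts to BP_Fossil01.
; It disables its own collision on BeginPlay.
; Its overlap handler casts to BP_Fossil01 and, if that piece's Piece1Correct returns true, shows the static mesh and re-enables collision.
; Its own Piece1Correct and Piece2Correct functions are stubs that always return false.
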(event `self.ReceiveBeginPlay`
  (`self.SetActorEnableCollision` false))

(event `self.ReceiveActorBeginOverlap`
  (params (OtherActor :type "Actor Object Reference"))
  (bind _asbp_fossil_01 (cast `/Game/_Blueprints/Puzzles/Bones/FossilPuzzle/BP_Fossil01` OtherActor))
  (bind _piece1correct (`/Game/_Blueprints/Puzzles/Bones/BPI_PuzzlePieces.Piece1Correct` _asbp_fossil_01))
  (if _piece1correct
    (`SceneComponent.SetVisibility` (`self.StaticMesh`) true false)
    (`self.SetActorEnableCollision` true)))

(fn `Piece1Correct`
  (returns (Piece1Correct :type Boolean))
  (return false))

(fn `Piece2Correct`
  (returns (Piece2Correct :type Boolean))
  (return false))

(fn `UserConstructionScript`)