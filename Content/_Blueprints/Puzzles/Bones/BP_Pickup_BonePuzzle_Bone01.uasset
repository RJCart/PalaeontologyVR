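; BP_Pickup_BonePuzzle_Bone01 is a bone pickup for the bone jigsaw puzzle, tied to the puzzle's first piece.
; On actor overlap it casts the other actor to BP_Puzzle_BoneJigsaw and reads Piece1IsCorrect.
; When that flag is true it hides its static mesh, without propagating to children, and prints a debug string.
; BeginPlay and Tick are disabled stubs, and construction only calls the parent.
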(event `self.ReceiveActorBeginOverlap`
  (params (OtherActor :type "Actor Object Reference"))
  (bind _asbp_puzzle_bone_jigsaw (cast `/Game/_Blueprints/Puzzles/Bones/BP_Puzzle_BoneJigsaw` OtherActor))
  (if (`/Game/_Blueprints/Puzzles/Bones/BP_Puzzle_BoneJigsaw.Piece1IsCorrect` _asbp_puzzle_bone_jigsaw)
    (`SceneComponent.SetVisibility` (`self.StaticMesh`) false false)
    (`KismetSystemLibrary.PrintString` "F")))

(fn `UserConstructionScript`
  (`parent.UserConstructionScript`))