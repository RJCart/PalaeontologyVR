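; Bone jigsaw puzzle Blueprint that detects specific pieces overlapping their slots.
; Three slot overlaps each flag the piece correct, reveal a bone mesh, play a drop sound, add score and create a level sequence player.
; PlaySequence plays an end sequence once the puzzle is complete, but neither it nor the five-piece completion check is called here.
; Several other helper functions are stubs or debug code.
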(event `self.ReceiveBeginPlay`
  (set `self.CurrentScore` 0.0))

(event `self.Piece1.OnComponentBeginOverlap`
  (params (OverlappedComponent :type "PrimitiveComponent Object Reference") (OtherActor :type "Actor Object Reference") (OtherComp :type "PrimitiveComponent Object Reference") (OtherBodyIndex :type Integer) (bFromSweep :type Boolean) (SweepResult :type "HitResult Structure (by ref)"))
  ; Insects
  (if (== OtherActor (`self.Piece1Reference`))
    (set `self.Piece1IsCorrect` true)
    (`GameplayStatics.PlaySound2D` (`self.DropSound`) 1.0 1.0 0.0 null null)
    (`SceneComponent.SetVisibility` (`self.SM_Bone_01`) true false)
    (set `self.Piece1Visibility` true)
    (`self.ScoreAdd`)
    (`LevelSequencePlayer.CreateLevelSequencePlayer` null)))

(event `self.Piece2.OnComponentBeginOverlap`
  (params (OverlappedComponent :type "PrimitiveComponent Object Reference") (OtherActor :type "Actor Object Reference") (OtherComp :type "PrimitiveComponent Object Reference") (OtherBodyIndex :type Integer) (bFromSweep :type Boolean) (SweepResult :type "HitResult Structure (by ref)"))
  ; Plants
  (if (== OtherActor (`self.Piece2Reference`))
    (set `self.Piece2IsCorrect` true)
    (`GameplayStatics.PlaySound2D` (`self.DropSound`) 1.0 1.0 0.0 null null)
    (`SceneComponent.SetVisibility` (`self.SM_Bone_02`) true false)
    (set `self.Piece2Visibility` true)
    (`self.ScoreAdd`)
    (`LevelSequencePlayer.CreateLevelSequencePlayer` null)))

(event `self.Piece3.OnComponentBeginOverlap`
  (params (OverlappedComponent :type "PrimitiveComponent Object Reference") (OtherActor :type "Actor Object Reference") (OtherComp :type "PrimitiveComponent Object Reference") (OtherBodyIndex :type Integer) (bFromSweep :type Boolean) (SweepResult :type "HitResult Structure (by ref)"))
  ; Scenery
  (if (== OtherActor (`self.Piece3Reference`))
    (set `self.Piece3IsCorrect` true)
    (`GameplayStatics.PlaySound2D` (`self.DropSound`) 1.0 1.0 0.0 null null)
    (`SceneComponent.SetVisibility` (`self.SM_Bone_03`) true false)
    (set `self.Piece3Visibility` true)
    (`self.ScoreAdd`)
    (`LevelSequencePlayer.CreateLevelSequencePlayer` null)))

(event `Play Sequence`
  ;[0.06339 0.07131 0.15 0.5] If All Pieces correct play end sequence
  (if (`self.IsPuzzleComplete`)
    (`LevelSequencePlayer.CreateLevelSequencePlayer` "/Game/_Art/Animation/AnimationSequence/QuetzalcoatlusSequences/LS_HouseFalling.LS_HouseFalling")
    (`MovieSceneSequencePlayer.Play` (`LevelSequenceActor.SequencePlayer` (`self.EndSequence`)))))

(fn `AdvancePuzzle`
  (bind _output_get (set `self.PuzzleStage` (+ (`self.PuzzleStage`) 1)))
  (`KismetSystemLibrary.PrintString` (`KismetStringLibrary.Conv_IntToString` _output_get)))

(fn `AllPiecesCorrect`
  (if (and (`self.Piece1IsCorrect`) (`self.Piece2IsCorrect`) (`self.Piece3IsCorrect`) (`self.Piece4IsCorrect`) (`self.Piece5IsCorrect`))
    (set `self.IsPuzzleComplete` true)))

(fn `IsPieceCorrect`
  (params (TestObject :type "Object Object Reference")))

(fn `Piece1Correct`
  (returns (Piece1Correct :type Boolean))
  (return false))

(fn `Piece2Correct`
  (returns (Piece2Correct :type Boolean))
  (return false))

(fn `PieceInPlace`
  (params (A :type "Object Object Reference") (B :type "Object Object Reference"))
  (if (== A B)
    (set `self.Piece1IsCorrect` true)))

(fn `PieceOutOfPlace`
  (params (A :type "Object Object Reference") (B :type "Object Object Reference"))
  (if (== A B)
    (set `self.Piece1IsCorrect` false)))

(fn `PuzzleWorldLocation`
  (params (PuzzleLocationIn :type "Vector Structure"))
  (returns (PuzzleLocationOut :type "Vector Structure"))
  (return (0.0 0.0 0.0)))

(fn `ScoreAdd`
  (set `self.CurrentScore` (+ (`self.CurrentScore`) (`self.AddScore`))))

(fn `Slot1Filled`
  (params (Slot1Filled :type Boolean))
  (returns (Slot1IsFilled :type Boolean))
  (return Slot1Filled))

(fn `UserConstructionScript`)