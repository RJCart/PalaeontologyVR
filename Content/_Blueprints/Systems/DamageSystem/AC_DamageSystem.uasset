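; Actor component that manages health, healing and damage for its owner, reporting outcomes through OnBlocked, OnDeath and OnDamageResponse dispatchers.
; TakeDamage routes each hit through the CanBeDamaged macro, which checks death, invincibility and blocking to choose damage, block or no damage.
; The DamageInfo CanBeDamaged flag bypasses invincibility, while CanBeBlocked is hardwired false, so blocking never triggers.
; Heal clamps to MaxHealth and only applies while alive.
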(fn `Heal`
  (params (HealAmount :type "Float (double-precision)"))
  (returns (NewHealth :type "Float (double-precision)"))
  ;[0.04205 0.05172 0.15 0.5] if is not dead
  (if (not (`self.IsDead`))
    ;[0.03913 0.05451 0.15 0.5] Heal, clamped to max health
    (bind _output_get (set `self.Health` (`KismetMathLibrary.FClamp` (+ HealAmount (`self.Health`)) 0.0 (`self.MaxHealth`))))
    (return _output_get)))

(fn `TakeDamage`
  (params (DamageInfo :type "/Game/_Blueprints/Systems/DamageSystem/S_DamageInfo Structure"))
  (returns (WasDamaged :type Boolean))
  (bind (_damageamount _damagetype _damageresponse _shoulddamagehit _canbedamaged) (break `/Game/_Blueprints/Systems/DamageSystem/S_DamageInfo` DamageInfo))
  (`self.CanBeDamaged` _canbedamaged
    (:`BlockDamage`
      (`self.OnBlocked`)
      (return false))
    (:`DoDamage`
      (bind _output_get (set `self.Health` (- (`self.Health`) _damageamount)))
      (if (<= _output_get 0.0)
        (set `self.IsDead` true)
        (`self.OnDeath`)
        (return true)
        (elif true
          (`self.OnDamageResponse` _damageresponse)
          (return true))))
    (:`NoDamage`
      (return false))))