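; Functional test that verifies the level's PlayerStart sits at its expected location.
; On StartTest it takes the first PlayerStart actor found and measures its distance from PlayerStartExpectedLocation.
; The test succeeds when that distance is within Tolerance and fails otherwise, reporting a message either way.
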(event `self.ReceiveStartTest`
  ;[0.02556 0.02935 0.15 0.5] Check playerstart is within a tolerance of it's desired start locaiton
  (bind _outactors (`GameplayStatics.GetAllActorsOfClass` "/Script/Engine.PlayerStart"))
  (if (<= (`KismetMathLibrary.VSize` (- (`self.K2_GetActorLocation` (`|GetArrayItem` _outactors)) (`self.PlayerStartExpectedLocation`))) (`self.Tolerance`))
    (`self.FinishTest` "Succeeded" "PlayerStart Correct")
    (else
      (`self.FinishTest` "Failed" "PlayerStart Incorrect"))))

(fn `UserConstructionScript`)